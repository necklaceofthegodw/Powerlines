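; Powerline actor that builds a row of pole meshes joined by cable components, regenerated in the construction script.
; Poles sit at spline points, which are first seeded in an evenly spaced straight line along the actor's forward vector.
; Same-named sockets on neighboring poles get cables sized to their distance, with stiffness taken from CableInfos.
; AddSplinePoints, uncalled here, adds evenly spaced points along a given line, carrying leftover length between calls.
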(event `self.ReceiveBeginPlay`)

(event `self.ReceiveTick`
  (params (DeltaSeconds :type "Float (single-precision)")))

(fn `AddPowerlineMeshToSpline`
  (params (PointIndex :type Integer) (MeshToAdd :type "StaticMesh Object Reference"))
  (returns (SpawnedMesh :type "StaticMeshComponent Object Reference"))
  (bind _spline (`self.Spline`))
  (bind _returnvalue (`AddComponent|NODE_AddStaticMeshComponent-1` :`RelativeTransform` (`KismetMathLibrary.Conv_VectorToTransform` (`SplineComponent.GetLocationAtSplinePoint` _spline PointIndex "Local"))))
  (`StaticMeshComponent.SetStaticMesh` _returnvalue MeshToAdd)
  (`SceneComponent.K2_SetRelativeRotation` _returnvalue (`SplineComponent.GetRotationAtSplinePoint` _spline PointIndex "Local") false false)
  (return _returnvalue))

(fn `AddSplinePoints`
  (params (LineStart :type "Vector Structure (by ref)") (LineEnd :type "Vector Structure"))
  (locals (PolesL :type Integer) (SpawnLocationL :type "Vector Structure" :default (0.0 0.0 0.0)) (DirectionL :type "Vector Structure") (LineLengthL :type "Float (double-precision)"))
  (bind _cablelength (`self.CableLength`))
  (set `local.DirectionL` (`KismetMathLibrary.Normal` (- LineEnd LineStart)))
  (bind _output_get (set `local.LineLengthL` (+ (`self.RemainingLineLength`) (`KismetMathLibrary.Vector_Distance` LineStart LineEnd))))
  (bind _output_get_2 (set `local.PolesL` (`KismetMathLibrary.FTrunc` (/ _output_get _cablelength))))
  (for _index (range 1 (+ _output_get_2 1))
    (set `local.SpawnLocationL` (+ (- LineStart (* (`local.DirectionL`) (`self.RemainingLineLength`))) (* (`local.DirectionL`) _cablelength _index)))
    (`SplineComponent.AddSplinePoint` (`self.Spline`) (`local.SpawnLocationL`) "World" true))
  (set `self.RemainingLineLength` (- (`local.LineLengthL`) (* (`local.PolesL`) (`self.CableLength`)))))

(fn `DestroyPowerlinesAndCables`
  (for _array_element (`self.PowerPoleMeshes`)
    (`SceneComponent.K2_DetachFromComponent` _array_element "KeepRelative" "KeepRelative" "KeepRelative" true)
    (`ActorComponent.K2_DestroyComponent` _array_element))
  (for _array_element_2 (`self.Cables`)
    (`SceneComponent.K2_DetachFromComponent` _array_element_2 "KeepRelative" "KeepRelative" "KeepRelative" true)
    (`ActorComponent.K2_DestroyComponent` _array_element_2))
  (`KismetArrayLibrary.Array_Clear` (`self.PowerPoleMeshes`))
  (`KismetArrayLibrary.Array_Clear` (`self.Cables`)))

(fn `SetCableProperties`
  (params (cableInfoToSet :type "/Game/Powerline/S_CableInfo Structure"))
  (bind ((`cable_2_4625BDA7482CAFDADE509BA4F8C4500B` _cable) (`cableLength_11_22CA21D740BE2F15DEFBA594A2E45F83` _cablelength) (`cableStiffness_17_9F86FB8C4EAC167F0CC929813472A8AC` _cablestiffness) (`endPoint_23_77B49BBC4F823B00B30F069B8355970E` _endpoint)) (break `/Game/Powerline/S_CableInfo` cableInfoToSet))
  (set `CableComponent.EndLocation` _endpoint _cable)
  (set `CableComponent.CableLength` _cablelength _cable)
  (set `CableComponent.SolverIterations` 10 _cable)
  (set `CableComponent.bEnableStiffness` _cablestiffness _cable))

(fn `SpawnPowerlineMeshesAlongSpline`
  (returns (OutPowerPoles :type "Array of StaticMeshComponent Object Reference"))
  (locals (PowerPolesL :type "Array of StaticMeshComponent Object Reference"))
  (if (`self.bInitialPolesSpawned`)
    ; Adding powerlinemeshes to new spline points
    (for _index (range (`SplineComponent.GetNumberOfSplinePoints` (`self.Spline`)))
      (bind _spawnedmesh (`self.AddPowerlineMeshToSpline` _index (`self.PowerlineMesh`)))
      (`KismetArrayLibrary.Array_Add` (`local.PowerPolesL`) _spawnedmesh))
    (else
      ; Initial spawn along a straight line
      (set `self.bInitialPolesSpawned` true)
      (`SplineComponent.ClearSplinePoints` (`self.Spline`) true)
      (for _index_2 (range (`self.InitialPolesNum`))
        (`SplineComponent.AddSplinePoint` (`self.Spline`) (+ (`self.K2_GetActorLocation`) (* (`self.GetActorForwardVector`) (`self.CableLength`) _index_2)) "World" true)
        (bind _spawnedmesh_2 (`self.AddPowerlineMeshToSpline` _index_2 (`self.PowerlineMesh`)))
        (`KismetArrayLibrary.Array_Add` (`local.PowerPolesL`) _spawnedmesh_2))))
  (return (`local.PowerPolesL`)))

(fn `UpdatePowerlines`
  (locals (CurrentIndexL :type Integer) (CurrentPoleMeshL :type "StaticMeshComponent Object Reference") (CurrentSocketNameL :type Name) (CurrentCableL :type "CableComponent Object Reference") (CableInfoL :type "Array of /Game/Powerline/S_CableInfo Structure"))
  (bind _currentsocketnamel (`local.CurrentSocketNameL`))
  (bind _returnvalue (`KismetMathLibrary.InverseTransformLocation` (`self.GetTransform`) (`SceneComponent.GetSocketLocation` (`local.CurrentPoleMeshL`) (`local.CurrentSocketNameL`))))
  (bind _output (`|GetArrayItem` (`self.PowerPoleMeshes`) (+ (`local.CurrentIndexL`) 1)))
  (bind _returnvalue_2 (`KismetMathLibrary.InverseTransformLocation` (`self.GetTransform`) (`SceneComponent.GetSocketLocation` _output (`local.CurrentSocketNameL`))))
  (`self.DestroyPowerlinesAndCables`)
  (bind _outpowerpoles (`self.SpawnPowerlineMeshesAlongSpline`))
  (bind _output_get (set `self.PowerPoleMeshes` _outpowerpoles))
  ;[1 1 1] Setup cables
  (for (_array_element _array_index) _output_get
    (set `local.CurrentPoleMeshL` _array_element)
    (set `local.CurrentIndexL` _array_index)
    (for _array_element_2 (`SceneComponent.GetAllSocketNames` (`local.CurrentPoleMeshL`))
      (set `local.CurrentSocketNameL` _array_element_2)
      (`/Engine/EditorBlueprintResources/StandardMacros.IsValid` _output
        (:`Is Valid`
          (bind _returnvalue_3 (`AddComponent|NODE_AddCableComponent-0` :`RelativeTransform` (`KismetMathLibrary.Conv_VectorToTransform` _returnvalue)))
          (bind _output_get_2 (set `local.CurrentCableL` _returnvalue_3))
          (`KismetArrayLibrary.Array_Add` (`self.Cables`) _output_get_2)
          (for _array_element_3 (`self.CableInfos`)
            (bind (_cable _splineposition _cablesocket _cablelength _cablestiffness) (break `/Game/Powerline/S_CableInfo` _array_element_3))
            (if (== _cablesocket _currentsocketnamel)
              (bind _s_cableinfo (make `/Game/Powerline/S_CableInfo` (`local.CurrentCableL`) (`local.CurrentIndexL`) _currentsocketnamel (`KismetMathLibrary.VSize` (- _returnvalue _returnvalue_2)) _cablestiffness _returnvalue_2))
              (`KismetArrayLibrary.Array_Add` (`local.CableInfoL`) _s_cableinfo)
              (`self.SetCableProperties` _s_cableinfo))))))))

(fn `UserConstructionScript`
  (`self.UpdatePowerlines`))